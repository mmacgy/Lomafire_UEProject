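; BP_EnemyAI is an enemy that chases the player once it spots a pawn, then removes itself after reaching them.
; PawnSensing sets a seeing flag, never cleared here, and calls FollowPlayer, which plays a camera shake at the player's location and runs AIMoveTo toward player 0.
; A successful move destroys the enemy after a short delay; the capsule overlap event is empty.
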(event OnSeePawn(PawnSensing)
  (params (Pawn :type Pawn%20Object%20Reference))
  (Variables|Default|SetisSeeingPlayer true)
  (CallFunction|FollowPlayer))

(event OnComponentBeginOverlap(CapsuleComponent)
  (params (OverlappedComponent :type Primitive%20Component%20Object%20Reference) (OtherActor :type Actor%20Object%20Reference) (OtherComp :type Primitive%20Component%20Object%20Reference) (OtherBodyIndex :type Integer) (bFromSweep :type Boolean) (SweepResult :type Hit%20Result%20Structure%20%28by%20ref%29)))

(event Custom|Follow%20Player
  (bind _returnvalue (Game|GetPlayerCharacter 0))
  (if (Variables|Default|GetisSeeingPlayer)
    (Camera|PlayWorldCameraShake "/Game/Blueprint/CamShake.CamShake_C" (Transformation|GetActorLocation _returnvalue) 0.0 5e+02)
    (AI|AIMoveTo self "0, 0, 0" _returnvalue 5.0 false
      (:OnSuccess
        (Utilities|FlowControl|Delay 0.5)
        (Actor|DestroyActor)))))

(event EventBeginPlay)

(event Collision|EventActorBeginOverlap
  (params (OtherActor :type Actor%20Object%20Reference)))

(event EventTick
  (params (DeltaSeconds :type Float%20%28single-precision%29)))

(fn ConstructionScript)