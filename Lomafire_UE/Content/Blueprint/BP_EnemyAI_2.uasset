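; Enemy AI pawn that chases the player on sight and damages them on reaching them.
; PawnSensing triggers FollowPlayer, which flags the player as chased, adds a chase audio component, shakes the camera and starts AIMoveTo toward the player.
; A successful move subtracts player HP and plays a damage sound.
; Tick polls the player character's Ending flag to stop the most recently added chase audio.
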(event OnSeePawn(PawnSensing)
  (params (Pawn :type Pawn%20Object%20Reference))
  ;[0.2965 0.6796 1] See Player
  (Variables|Default|SetisSeeingPlayer true)
  (CallFunction|FollowPlayer))

(event Custom|Follow%20Player
  (bind _returnvalue (Game|GetPlayerCharacter 0))
  ;[1 0.2879 0.3577] Mechanic
  (if (Variables|Default|GetisSeeingPlayer)
    (bind _asbp_third_person_character (Utilities|Casting|CastToBP_ThirdPersonCharacter _returnvalue))
    (Variables|/Game/ThirdPerson/Blueprints/BP_ThirdPersonCharacter.BP_ThirdPersonCharacter_C|SetBeingChased? _asbp_third_person_character true)
    (bind _returnvalue_2 (AddComponent|AddAudioComponent false))
    (Variables|Default|SetChase _returnvalue_2)
    (Camera|PlayWorldCameraShake "/Game/Blueprint/CamShake.CamShake_C" (Transformation|GetActorLocation _returnvalue) 0.0 5e+02)
    (AI|AIMoveTo self "0, 0, 0" _returnvalue 5.0 false
      (:OnSuccess
        (bind _asbp_third_person_character_2 (Utilities|Casting|CastToBP_ThirdPersonCharacter _returnvalue))
        (Variables|/Game/ThirdPerson/Blueprints/BP_ThirdPersonCharacter.BP_ThirdPersonCharacter_C|SetPlayer_HP _asbp_third_person_character_2 (- (Variables|/Game/ThirdPerson/Blueprints/BP_ThirdPersonCharacter.BP_ThirdPersonCharacter_C|GetPlayer_HP _asbp_third_person_character_2) 1e+01))
        (Audio|PlaySound2D "/Game/Sound/DamageTaken_Cue.DamageTaken_Cue" 1.0 1.0 0.0 0 0)))))

(event EventTick
  (params (DeltaSeconds :type Float%20%28single-precision%29))
  ;[1 0.9404 0.4792] Ending Check
  (bind _asbp_third_person_character (Utilities|Casting|CastToBP_ThirdPersonCharacter (Game|GetPlayerCharacter 0)))
  (if (Variables|/Game/ThirdPerson/Blueprints/BP_ThirdPersonCharacter.BP_ThirdPersonCharacter_C|GetEnding? _asbp_third_person_character)
    (Audio|Components|Audio|Stop (Variables|Default|GetChase))))

(fn ConstructionScript)